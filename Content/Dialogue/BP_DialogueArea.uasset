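; BP_DialogueArea is a trigger area that lets the player read an NPC's dialogue on screen.
; BeginPlay caches the data table rows matching its NPCID.
; Player overlap shows an interact popup, and leaving removes it and any open dialogue.
; Each Interact advances the line counter and displays the row matching ConversationID and line, closing and resetting unless exactly one line is collected.
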(event OnComponentEndOverlap(DialogueTriggerableRange)
  (params (OverlappedComponent :type Primitive%20Component%20Object%20Reference) (OtherActor :type Actor%20Object%20Reference) (OtherComp :type Primitive%20Component%20Object%20Reference) (OtherBodyIndex :type Integer))
  (bind _interactbutton (Variables|Default|GetInteractButton))
  (Utilities|Casting|CastToBP_ThirdPersonCharacterCustom OtherActor)
  (Utilities|IsValid _interactbutton
    (:Is%20Valid
      (Widget|RemovefromParent _interactbutton)
      (Utilities|IsValid (Variables|Default|GetDialogueWidget)
        (:Is%20Valid
          (Widget|RemovefromParent (Variables|Default|GetDialogueWidget))
          (Variables|Default|SetDialogueWidget 0)
          (Variables|Default|SetLineCurrent 0))))))

(event OnComponentBeginOverlap(DialogueTriggerableRange)
  (params (OverlappedComponent :type Primitive%20Component%20Object%20Reference) (OtherActor :type Actor%20Object%20Reference) (OtherComp :type Primitive%20Component%20Object%20Reference) (OtherBodyIndex :type Integer) (bFromSweep :type Boolean) (SweepResult :type Hit%20Result%20Structure%20%28by%20ref%29))
  (Utilities|Casting|CastToBP_ThirdPersonCharacterCustom OtherActor)
  (bind _returnvalue (UserInterface|CreateWidget "/Game/Dialogue/WBP_InteractPopUp.WBP_InteractPopUp_C"))
  (bind _output_get (Variables|Default|SetInteractButton _returnvalue))
  (UserInterface|Viewport|AddtoViewport _output_get 0))

(event EventBeginPlay
  (bind _outrownames (DataTable|GetDataTableRowNames "/Game/Dialogue/Game1Start_Dialogue_CSV_-_Dialogue.Game1Start_Dialogue_CSV_-_Dialogue"))
  (for _array_element _outrownames
    (bind _returnvalue (Utilities|GetDataTableRow "/Game/Dialogue/Game1Start_Dialogue_CSV_-_Dialogue.Game1Start_Dialogue_CSV_-_Dialogue" _array_element)
      (:then
        (if (== (Variables|Default|GetNPC_ID) (.NPC_ID (Utilities|Struct|BreakDTS_Dialogue _returnvalue)))
          (Utilities|Array|Add (Variables|Default|GetMyDialogue) _array_element))))))

(event EventInteract
  (bind _interactbutton (Variables|Default|GetInteractButton))
  (Math|Integer|IncrementInt (Variables|Default|GetLineCurrent)
    (:%20%20
      (CallFunction|DialogueCreate)
      (Utilities|IsValid _interactbutton
        (:Is%20Valid
          (Widget|RemovefromParent _interactbutton))))))

(fn ConstructionScript)

(fn DialogueCreate
  (Utilities|IsValid (Variables|Default|GetDialogueWidget)
    (:Is%20Valid
      (bind _line (CallFunction|GetDialogueLine))
      (Utilities|IsValid (Variables|Default|GetDialogueWidget)
        (:Is%20Valid
          (Variables|/Game/Dialogue/WBP_Dialogue.WBP_Dialogue_C|SetDialogueText (Variables|Default|GetDialogueWidget) _line))))
    (:Is%20Not%20Valid
      (bind _returnvalue (UserInterface|CreateWidget "/Game/Dialogue/WBP_Dialogue.WBP_Dialogue_C" (Game|GetPlayerController 0)))
      (bind _output_get (Variables|Default|SetDialogueWidget _returnvalue))
      (UserInterface|Viewport|AddtoViewport _output_get 0)
      (bind _line_2 (CallFunction|GetDialogueLine))
      (Variables|/Game/Dialogue/WBP_Dialogue.WBP_Dialogue_C|SetDialogueText (Variables|Default|GetDialogueWidget) _line_2))))

(fn GetDialogueLine
  (for _array_element (Variables|Default|GetMyDialogue)
    (bind _returnvalue (Utilities|GetDataTableRow "/Game/Dialogue/Game1Start_Dialogue_CSV_-_Dialogue.Game1Start_Dialogue_CSV_-_Dialogue" _array_element)
      (:then
        (if (and (== (.Conversation_ID (Utilities|Struct|BreakDTS_Dialogue _returnvalue)) (Variables|Default|GetConversation_ID)) (== (.Line_ID (Utilities|Struct|BreakDTS_Dialogue _returnvalue)) (Variables|Default|GetLineCurrent)))
          (Utilities|Array|Add (LocalVariables|GetReturned%20Lines) (.Dialogue (Utilities|Struct|BreakDTS_Dialogue _returnvalue)))))))
  (if (== (Utilities|Array|Length (LocalVariables|GetReturned%20Lines)) 1)
    (return (Utilities|Array|Get(acopy) (LocalVariables|GetReturned%20Lines)))
    (else
      (Widget|RemovefromParent (Variables|Default|GetDialogueWidget))
      (Variables|Default|SetDialogueWidget 0)
      (Variables|Default|SetLineCurrent 0))))