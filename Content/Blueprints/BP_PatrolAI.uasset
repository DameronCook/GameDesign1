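; Patrol AI character that walks between tagged BP_PatrolPoint actors at a walk speed randomized on BeginPlay.
; BeginPlay gathers and shuffles the points, then GoToPatrolPoint loops through AI moves, pausing after each success or failure.
; The point list reshuffles after each full pass.
; A separate MoveTo event repeatedly chases the player with the same retry delay, but nothing in this Blueprint calls it.
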(event Custom|GoToPatrolPoint
  (AI|AIMoveTo self (Transformation|GetActorLocation (Utilities|Array|Get(acopy) (stale EventBeginPlay _outactors) (Variables|Default|GetIndex))) 0 2e+02 false
    (:OnSuccess
      _)
    (:OnFail
      _))
  (bind _result (Math|Integer|IncrementInt (Variables|Default|GetIndex))
    (:%20%20
      (if (>= _result (Utilities|Array|Length (stale EventBeginPlay _outactors)))
        (Variables|Default|SetIndex 0)
        (Utilities|Array|Shuffle (stale EventBeginPlay _outactors)))
      (Utilities|FlowControl|Delay 2.0)
      (CallFunction|GotoPatrolPoint))))

(event Custom|MoveTo
  (AI|AIMoveTo self "0, 0, 0" (Game|GetPlayerCharacter 0) 2e+02 false
    (:OnSuccess
      _)
    (:OnFail
      _))
  (Utilities|FlowControl|Delay 2.0)
  (CallFunction|Moveto))

(event EventBeginPlay
  (bind _outactors (Actor|GetAllActorsOfClasswithTag "/Game/Blueprints/BP_PatrolPoint.BP_PatrolPoint_C" (Variables|Default|GetPatrolPointTag)))
  (Utilities|Array|Shuffle _outactors)
  (Development|PrintString (Utilities|String|Append "There are: " (Utilities|String|ToString(Integer) (Utilities|Array|Length _outactors)) " patrol points"))
  (CallFunction|GotoPatrolPoint)
  (Variables|/Script/Engine.CharacterMovementComponent|SetMaxWalkSpeed (Variables|Character|GetCharacterMovement) (* (Math|Random|RandomIntegerinRange 8 12) 25.0)))

(fn ConstructionScript)