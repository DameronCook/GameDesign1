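; BP_KillingFloor is a lava-themed hazard that sends the player back to a checkpoint on contact.
; Overlapping the Cube casts to BP_ThirdPersonCharacterCustom, calls its LoadCheckpoint, then plays the lava flow sound at the floor's location.
; The same sound also plays on BeginPlay, alongside a debug print of the location, and whenever anything begins overlapping the Sphere.
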(event OnComponentBeginOverlap(Cube)
  (params (OverlappedComponent :type Primitive%20Component%20Object%20Reference) (OtherActor :type Actor%20Object%20Reference) (OtherComp :type Primitive%20Component%20Object%20Reference) (OtherBodyIndex :type Integer) (bFromSweep :type Boolean) (SweepResult :type Hit%20Result%20Structure%20%28by%20ref%29))
  (bind _asbp_third_person_character_custom (Utilities|Casting|CastToBP_ThirdPersonCharacterCustom OtherActor))
  (Default|LoadCheckpoint _asbp_third_person_character_custom)
  (Audio|PlaySoundatLocation "/Game/Audio/Lava_Flow_Sound_Effect_Cue.Lava_Flow_Sound_Effect_Cue" (Transformation|GetActorLocation) "0, 0, 0" 1.0 1.0 0.0 0 0 0 0))

(event OnComponentBeginOverlap(Sphere)
  (params (OverlappedComponent :type Primitive%20Component%20Object%20Reference) (OtherActor :type Actor%20Object%20Reference) (OtherComp :type Primitive%20Component%20Object%20Reference) (OtherBodyIndex :type Integer) (bFromSweep :type Boolean) (SweepResult :type Hit%20Result%20Structure%20%28by%20ref%29))
  (Audio|PlaySoundatLocation "/Game/Audio/Lava_Flow_Sound_Effect_Cue.Lava_Flow_Sound_Effect_Cue" (Transformation|GetActorLocation) "0, 0, 0" 1.0 1.0 0.0 0 0 0 0))

(event EventBeginPlay
  (bind _returnvalue (Transformation|GetActorLocation))
  (Audio|PlaySoundatLocation "/Game/Audio/Lava_Flow_Sound_Effect_Cue.Lava_Flow_Sound_Effect_Cue" _returnvalue "0, 0, 0" 1.0 1.0 0.0 0 0 0 0)
  (Development|PrintString (Utilities|String|ToString(Vector) _returnvalue)))

(fn ConstructionScript)