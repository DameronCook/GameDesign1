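; Finish-line actor that times laps for the custom third-person character.
; On BeginPlay it adds a timer widget to the viewport and starts a self-calling Delay loop that refreshes the current lap time on screen and as debug text.
; When the character overlaps the box, it prints the lap time and resets the timestamp that all times are measured from, using real-time seconds.
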(event OnComponentBeginOverlap(Box)
  (params (OverlappedComponent :type Primitive%20Component%20Object%20Reference) (OtherActor :type Actor%20Object%20Reference) (OtherComp :type Primitive%20Component%20Object%20Reference) (OtherBodyIndex :type Integer) (bFromSweep :type Boolean) (SweepResult :type Hit%20Result%20Structure%20%28by%20ref%29))
  (Utilities|Casting|CastToBP_ThirdPersonCharacterCustom OtherActor)
  (Development|PrintString (Utilities|String|Append "Lap Time: " (Utilities|String|ToString(Text) (Utilities|Text|ToText(Float) (- (Utilities|Time|GetRealTimeSeconds) (Variables|Default|GetLastTimeStamp)) "HalfToEven" false true 1 324 0 1)) " seconds"))
  (Variables|Default|SetLastTimeStamp (Utilities|Time|GetRealTimeSeconds)))

(event Custom|OnScreenTimer
  (bind _returnvalue (Utilities|Time|GetRealTimeSeconds))
  (bind _lasttimestamp (Variables|Default|GetLastTimeStamp))
  (bind _returnvalue_2 (- _returnvalue _lasttimestamp))
  (bind _returnvalue_3 (Utilities|Text|ToText(Float) _returnvalue_2 "HalfToEven" false true 1 324 0 1))
  (bind _returnvalue_4 (Utilities|String|ToString(Text) _returnvalue_3))
  (bind _returnvalue_5 (Utilities|String|Append "Current Lap Time: " _returnvalue_4))
  (Development|PrintString _returnvalue_5 true true "(R=0.000000,G=0.660000,B=1.000000,A=1.000000)" 0.1)
  (Variables|/Script/UMG.TextBlock|SetText (Variables|/Game/Widgets/WBP_FinishLineTimer.WBP_FinishLineTimer_C|GetCurrentTimeText (Variables|Default|GetWBP_FinishLineTimer)) (Utilities|Text|ToText(String) _returnvalue_5))
  (Utilities|FlowControl|Delay 0.1)
  (CallFunction|OnScreenTimer))

(event EventBeginPlay
  (bind _returnvalue (UserInterface|CreateWidget "/Game/Widgets/WBP_FinishLineTimer.WBP_FinishLineTimer_C"))
  (bind _output_get (Variables|Default|SetWBP_FinishLineTimer _returnvalue))
  (UserInterface|Viewport|AddtoViewport _output_get 0)
  (CallFunction|OnScreenTimer))

(fn ConstructionScript)